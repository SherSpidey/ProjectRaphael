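; Raphael particle Blueprint (BR variant) for a magnet particle that either takes control of an actor or equips onto the player.
; For control, a timeline moves it to the controlled actor, then triggers magnet control and particle death.
; When equipped, it binds a Niagara effect to the player's skeletal mesh, flies to the player, hides its mesh and scales the effect up.
; Destroying the equipped particle reverses that scale before death.
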(event EventSpecialFunction
  (bind _controlparticle (Variables|Default|GetControlParticle))
  (bind _particlestate (Variables|Default|GetParticleState))
  ;[1 1 1] Equip Particle
  (if (Utilities|Enum|Equal(Enum) _particlestate "EPS_Function")
    (|CallParentFunction)
    (if (Utilities|Enum|Equal(Enum) _particlestate "EPS_Equipped")
      (bind _playercharacter (Variables|Default|GetPlayerCharacter)
        (:then
          (Class|NiagaraFunctionLibrary|OverrideSystemUserVariableSkeletalMeshComponent _controlparticle "PlayerMesh" (Actor|GetComponentbyClass _playercharacter "/Script/Engine.SkeletalMeshComponent"))
          (Class|RaphaelParticleBR|SetControlParticleMaterial)
          (Components|Activation|SetActive _controlparticle true false)
          (bind _locationalpha (Timeline|EquippedTimeline PlayFromStart)
            (:Update
              (Transformation|SetActorLocation (Math|Vector|Lerp(Vector) (Variables|Default|GetStartLocation) (Transformation|GetActorLocation (Variables|Default|GetPlayerCharacter)) _locationalpha) false false))
            (:Finished
              (Rendering|SetVisibility (Variables|Default|GetParticleMesh) false false)
              (Components|Timeline|PlayfromStart (Variables|Default|GetScaleTimeline)))))
        (:else)))))

(event EventDestroyEquippedParticle
  ;[1 1 1] Equip Particle
  (|CallParentFunction)
  (Components|Timeline|ReversefromEnd (Variables|Default|GetScaleTimeline)))

(event EventBeginControl
  ;[1 1 1] Control magnet
  (Variables|Default|GetControlledActor
    (:then
      (bind _positionalpha (Timeline|ControlTimeline Play)
        (:Update
          (Transformation|SetActorLocation (Math|Vector|Lerp(Vector) (Variables|Default|GetStartLocation) (Transformation|GetActorLocation (Variables|Default|GetControlledActor)) _positionalpha) false false))
        (:Finished
          (Class|RaphaelParticleBR|ControlMagnet)
          (Class|RaphaelParticle|OnParticlePendingKill)
          (Class|RaphaelParticle|ParticleDeath))))
    (:else)))

(fn ConstructionScript
  (Class|RaphaelParticleBR|SetParticleMagnet))