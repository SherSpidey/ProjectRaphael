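; Magnet actor that displays its magnetic pole type through the material on its mesh.
; The construction script sets the mesh material for North, South or Iron from the PoleType variable.
; A SetMagnetPoleType event changes the pole at runtime and swaps the material, though it handles only North and South, leaving Iron's material unapplied.
; It contains no force or attraction logic.
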(event EventBeginPlay)

(event Collision|EventActorBeginOverlap
  (params (OtherActor :type Actor%20Object%20Reference)))

(event EventSetMagnetPoleType
  (params (NewPoleType :type EMagnetPoleType%20Enum :default "EMT_North"))
  (bind _magnetmesh (Variables|Default|GetMagnetMesh))
  (bind _output_get (Variables|Default|SetPoleType NewPoleType))
  (switch Utilities|FlowControl|Switch|SwitchonEMagnetPoleType _output_get
    (:EMT_North
      (Rendering|Material|SetMaterial _magnetmesh 0 "/Game/Asset/Material/PoleNorth.PoleNorth"))
    (:EMT_South
      (Rendering|Material|SetMaterial _magnetmesh 0 "/Game/Asset/Material/PoleSouth.PoleSouth"))))

(fn ConstructionScript
  (bind _magnetmesh (Variables|Default|GetMagnetMesh))
  (switch Utilities|FlowControl|Switch|SwitchonEMagnetPoleType (Variables|Default|GetPoleType)
    (:EMT_North
      (Rendering|Material|SetMaterial _magnetmesh 0 "/Game/Asset/Material/PoleNorth.PoleNorth"))
    (:EMT_South
      (Rendering|Material|SetMaterial _magnetmesh 0 "/Game/Asset/Material/PoleSouth.PoleSouth"))
    (:EMT_Iron
      (Rendering|Material|SetMaterial _magnetmesh 0 "/Game/Asset/Geometry/Meshes/CubeMaterial.CubeMaterial"))))