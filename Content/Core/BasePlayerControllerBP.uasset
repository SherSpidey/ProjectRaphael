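; Base player controller that relays gameplay UI requests to the HUD.
; Custom events forward crosshair scale, crosshair visibility and restart display toggles, each casting the HUD before calling it.
; The CheckGuide input shows the guide while held and hides it on release.
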(event EventBeginPlay)

(event EventTick
  (params (DeltaSeconds :type Float%20%28single-precision%29)))

(event EventSetCrossHairDynamic
  (params (Scale :type Float%20%28single-precision%29))
  (bind _ashud (Utilities|Casting|CastToHUD (Variables|Default|GetHUD)))
  (Default|UpdateCrossHair _ashud Scale))

(event EventSetHUDVisibility
  (params (Enable :type Boolean))
  (bind _ashud (Utilities|Casting|CastToHUD (Variables|Default|GetHUD)))
  (Default|SetCrossHairVisibility _ashud Enable))

(event EventShowRestart
  (params (Enable :type Boolean))
  (bind _ashud (Utilities|Casting|CastToHUD (Variables|Default|GetHUD)))
  (Default|SetRestart _ashud Enable))

(event Input|ActionEvents|InputActionCheckGuide
  (params (Key :type Key%20Structure :default "None"))
  (bind _hud (Variables|Default|GetHUD))
  (:Pressed
    (bind _ashud (Utilities|Casting|CastToHUD _hud))
    (Default|SetGuide _ashud true))
  (:Released
    (bind _ashud_2 (Utilities|Casting|CastToHUD _hud))
    (Default|SetGuide _ashud_2 false)))

(fn ConstructionScript)