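; RaphaelParticleSilverBP is the silver Raphael particle, a child Blueprint that extends its parent's activate and return-to-player behavior.
; On activation it spawns a silver particle pawn as ControllerPawn, aligns its camera boom to the player's control rotation and plays a scale timeline.
; That timeline scales the mesh toward ParticleRadius and reverses on return to the player.
; Holding jump runs a second timeline that ramps JumpPower from initial to maximum.
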(event EventParticleActive
  (bind _returnvalue (Game|SpawnActorfromClass "/Game/Character/ParticlePawn/RaphaelParticleSilverPawn.RaphaelParticleSilverPawn_C" (Math|Transform|MakeTransform "0, 0, 0" "0, 0, 0" "1,1,1") "AlwaysSpawn" 0 0))
  (bind _output_get (Variables|Default|SetControllerPawn _returnvalue))
  (Class|RaphaelParticle|GetPlayerCharacter)
  (bind _playercharacter (Variables|Default|GetPlayerCharacter)
    (:then
      (Transformation|SetWorldRotation (Variables|/Script/ProjectRaphael.RaphaelParticlePawn|GetCameraBoom _output_get) (Pawn|GetControlRotation _playercharacter :!class /Script/Engine.Pawn) false false)
      (|CallParentFunction)
      (Components|Timeline|PlayfromStart (Variables|Default|GetScaleTimeLine)))
    (:else)))

(event EventBacktoPlayer
  (|CallParentFunction)
  (Utilities|String|Reverse (Variables|Default|GetScaleTimeLine)))

(event EventJumpHold
  (bind _forcealpha (Timeline|JumpForceTimeLine PlayFromStart)
    (:Update
      (Variables|Default|SetJumpPower (Math|Float|Lerp (Variables|Default|GetJumpInitPower) (Variables|Default|GetJumpMaxPower) _forcealpha)))))

(fn ConstructionScript)