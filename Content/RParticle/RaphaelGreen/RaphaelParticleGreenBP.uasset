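; RaphaelParticleGreenBP is a particle actor that previews the trajectory it would follow if launched along the player's camera view.
; ShowTrail runs a projectile path prediction from the actor's location with a fixed launch speed, ignoring itself and the player and drawing one-frame debug.
; The predicted positions replace TrailSpline's points, passed as local space although the prediction returns world positions.
; It contains no launch logic, and ThrowForce is unused.
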(event EventShowTrail
  (bind _playercharacter (Variables|Default|GetPlayerCharacter)
    (:then
      (Spline|ClearSplinePoints (Variables|Default|GetTrailSpline) true)
      (bind _outpathpositions (Class|GameplayStatics|BlueprintPredictProjectilePathbyTraceChannel (Transformation|GetActorLocation) (* (Math|Vector|GetForwardVector (Variables|/Script/ProjectRaphael.BaseCharacter|GetFollowCamera _playercharacter)) 1e+03) true (Variables|Default|GetParticleRadius) "ECC_WorldDynamic" false (Utilities|Array|MakeArray self (Variables|Default|GetPlayerCharacter)) "ForOneFrame"))
      (Spline|SetSplinePoints (Variables|Default|GetTrailSpline) _outpathpositions "Local" true))
    (:else)))

(fn ConstructionScript)