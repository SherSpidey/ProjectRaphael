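; Raphael's black particle, which takes physics-handle control of a target static mesh actor.
; On activation it flies to the target on a timeline, calls Transformer partway, then grabs the mesh and runs ControlTarget on a looping timer.
; While controlling, the function input eases the hold distance in and out; reactivating damps velocity, releases, applies press force and fades the particle.
; Niagara variables bind the target mesh and drive the death scale.
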(event Custom|StartControl
  ;[1 1 1] Active Funciton
  (Class|RaphaelParticleBlack|ControlTarget))

(event EventBeginPlay)

(event Collision|EventActorBeginOverlap
  (params (OtherActor :type Actor%20Object%20Reference)))

(event EventTick
  (params (DeltaSeconds :type Float%20%28single-precision%29)))

(event EventControlParticleInit
  ;[1 1 1] Particle init
  (bind _targetactor (Variables|Default|GetTargetActor)
    (:then
      (bind _asstatic_mesh_component (Utilities|Casting|CastToStaticMeshComponent (Variables|/Script/Engine.Actor|GetRootComponent _targetactor)))
      (Class|NiagaraFunctionLibrary|OverrideSystemUserVariableStaticMeshComponent (Variables|Default|GetControlParticle) "TargetMesh" _asstatic_mesh_component)
      (|CallParentFunction))
    (:else)))

(event EventParticleActive
  (bind _targetactor (Variables|Default|GetTargetActor))
  ;[1 1 1] Active Funciton
  (switch Utilities|FlowControl|Switch|SwitchonEBlackParticleState (Variables|Default|GetParticleState)
    (:EPS_Idle
      (Class|RaphaelParticleBlack|GetTargetActor)
      (Variables|Default|GetTargetActor
        (:then
          (|CallParentFunction)
          (Class|RaphaelParticle|OnParticlePendingActive)
          (Variables|Default|SetParticleState "EPS_Moving")
          (Class|RaphaelParticleBlack|CalculateSpeed (Components|Timeline|GetTimelineLength (Variables|Default|GetControlTimeLine)))
          (bind _movealpha (Timeline|ControlTimeLine PlayFromStart)
            (:Update
              (Utilities|FlowControl|Sequence
                (:then_0
                  (Transformation|SetActorLocation (Math|Vector|Lerp(Vector) (Variables|Default|GetStartPosition) (Transformation|GetActorLocation (Variables|Default|GetTargetActor)) _movealpha) false false))
                (:then_1
                  (if (>= _movealpha 0.3)
                    (Utilities|FlowControl|DoOnce false
                      (:Completed
                        (Class|RaphaelParticleBlack|Transformer)))))))
            (:Finished
              (Utilities|Time|SetTimerbyEvent (delegate Custom|StartControl) 0.001 true)
              (Class|NiagaraComponent|SetVariableBool (Variables|Default|GetControlParticle) "bInstant" true)
              (bind _asstatic_mesh_component (Utilities|Casting|CastToStaticMeshComponent (Variables|/Script/Engine.Actor|GetRootComponent (Variables|Default|GetTargetActor))))
              (Physics|Components|PhysicsHandle|GrabComponentatLocationwithRotation (Variables|Default|GetControlHandle) _asstatic_mesh_component "None" (.location (Transformation|GetWorldTransform _asstatic_mesh_component)) (.rotation (Transformation|GetWorldTransform _asstatic_mesh_component)))
              (Variables|Default|SetParticleState "EPS_Control"))))
        (:else)))
    (:EPS_Control
      (bind _asstatic_mesh_component_2 (Utilities|Casting|CastToStaticMeshComponent (Variables|/Script/Engine.Actor|GetRootComponent _targetactor)))
      (Physics|SetPhysicsLinearVelocity _asstatic_mesh_component_2 (* (Transformation|GetVelocity _targetactor) 0.1) false "None")
      (Physics|Components|PhysicsHandle|ReleaseComponent (Variables|Default|GetControlHandle))
      (Class|RaphaelParticle|OnParticlePendingKill)
      (Class|RaphaelParticleBlack|ApplyPressForce)
      (Class|RaphaelParticleBlack|ControlParticleDeath))))

(event EventParticleSetFunctionEnable
  (params (Enabled :type Boolean))
  (bind _controldistance (Variables|Default|GetControlDistance))
  ;[1 1 1] Update
  (if (Utilities|Enum|Equal(Enum) (Variables|Default|GetParticleState) "EPS_Control")
    (if Enabled
      (bind _holdalpha (Timeline|HoldTimeLine Play)
        (:Update
          (Variables|Default|SetCurrentDistance (Math|Float|Lerp _controldistance (- _controldistance (Variables|Default|GetControlPressDistance)) _holdalpha))))
      (else
        (Timeline|HoldTimeLine Reverse)))))

(event EventControlParticleDeath
  ;[1 1 1] Particle death
  (bind _scalealpha (Timeline|ParticleDeathTimeLine PlayFromStart)
    (:Update
      (Niagara|SetNiagaraVariable(Float) (Variables|Default|GetControlParticle) "ScaleAlpha" _scalealpha))
    (:Finished
      (Class|RaphaelParticleBlack|OnControlParticleDeathFinish))))

(fn ConstructionScript)